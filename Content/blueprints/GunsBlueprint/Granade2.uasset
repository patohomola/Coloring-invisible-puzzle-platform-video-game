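; Grenade actor that bursts into a spray of bullet raycasts after a two-second fuse from BeginPlay.
; A loop calls BulletRaycast about a hundred times from Sphere1's location, each along a random vector scaled by Pi.
; The short Delay ending the loop body does not pause a standard ForLoop, so the rays fire together.
; Overlap and Tick only call the parent, and a random-color node is unused.
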(event `self.ReceiveBeginPlay`
  (`parent.ReceiveBeginPlay`)
  (`KismetSystemLibrary.Delay` 2.0)
  (for _ (range 101)
    (`self.BulletRaycast` (`SceneComponent.K2_GetComponentLocation` (`self.Sphere1`)) (* (`KismetMathLibrary.MakeVector` (`KismetMathLibrary.RandomFloatInRange` -1.0 1.0) (`KismetMathLibrary.RandomFloatInRange` -1.0 1.0) (`KismetMathLibrary.RandomFloatInRange` -1.0 1.0)) (`KismetMathLibrary.GetPI`)))
    (`KismetSystemLibrary.Delay` 0.1)))

(event `self.ReceiveActorBeginOverlap`
  (params (OtherActor :type "Actor Object Reference"))
  (`parent.ReceiveActorBeginOverlap` null))

(event `self.ReceiveTick`
  (params (DeltaSeconds :type "Float (single-precision)"))
  (`parent.ReceiveTick` 0.0))

(fn `UserConstructionScript`
  (`parent.UserConstructionScript`))