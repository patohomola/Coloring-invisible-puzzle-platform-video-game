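; GenerateMaze is an early maze generator that so far only sets up wall storage for a Height by Width grid.
; On BeginPlay, Init clears and resizes the NodesWhichContainWall array, then a loop over Width runs an empty sequence, so no maze is built.
; Helper functions read and write cells by flattening two coordinates into a row-major index.
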(event `self.ReceiveBeginPlay`
  (`self.Init`)
  (for _ (range (+ (`self.Width`) 1))
    (`|ExecutionSequence`)))

(fn `arrayIndexFromDimension`
  (params (A :type Integer) (B :type Integer))
  (returns (NewParam :type Integer))
  (return (+ (* A (`self.Width`)) B)))

(fn `Init`
  (bind _nodeswhichcontainwall (`self.nodesWhichContainWall`))
  (bind _output_get (set `self.ArraySize` (* (`self.height`) (`self.Width`))))
  (`KismetArrayLibrary.Array_Clear` _nodeswhichcontainwall)
  (`KismetArrayLibrary.Array_Resize` _nodeswhichcontainwall _output_get))

(fn `readFromArray`
  (params (A :type Integer) (B :type Integer))
  (returns (Output :type Boolean))
  (bind _newparam (`self.arrayIndexFromDimension` A B))
  (return (`|GetArrayItem` (`self.nodesWhichContainWall`) _newparam)))

(fn `Set2array`
  (params (A :type Integer) (B :type Integer) (Item :type "Boolean (by ref)"))
  (bind _newparam (`self.arrayIndexFromDimension` A B))
  (`KismetArrayLibrary.Array_Set` (`self.nodesWhichContainWall`) _newparam Item))

(fn `UserConstructionScript`)