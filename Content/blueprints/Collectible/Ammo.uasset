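; Ammo pickup collectible that adds rounds to the PlayerPainter's equipped gun.
; On Tick, while the player's MagnetON flag is set and the player is within range, it moves toward them at constant speed by setting its transform without sweep.
; Any overlap with its Box grants the ammo to the player pawn without checking the overlapping actor, then destroys the pickup and plays a 2D sound.
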(event `self.ReceiveBeginPlay`
  (bind _asplayer_painter (cast `/Game/blueprints/GameCharacter/PlayerPainter` (`GameplayStatics.GetPlayerPawn` 0)))
  (set `self.As Player Painter` _asplayer_painter))

(event `self.ReceiveTick`
  (params (DeltaSeconds :type "Float (single-precision)"))
  (bind (_returnvalue_location _returnvalue_rotation _returnvalue_scale) (`KismetMathLibrary.BreakTransform` (`self.GetTransform` self)))
  (bind _returnvalue (`self.K2_GetActorLocation` (`GameplayStatics.GetPlayerPawn` 0)))
  (bind _returnvalue_2 (`self.K2_GetActorLocation` self))
  (if (`/Game/blueprints/GameCharacter/PlayerPainter.MagnetON` (`self.As Player Painter`))
    (if (> 2000.0 (`KismetMathLibrary.Vector_Distance` _returnvalue_2 _returnvalue))
      (`self.K2_SetActorTransform` (`KismetMathLibrary.MakeTransform` (+ (* (`KismetMathLibrary.Normal` (- _returnvalue _returnvalue_2)) (`GameplayStatics.GetWorldDeltaSeconds`) 1000.0) _returnvalue_location) _returnvalue_rotation _returnvalue_scale)))))

(event `self.Box.OnComponentBeginOverlap`
  (params (OverlappedComponent :type "PrimitiveComponent Object Reference") (OtherActor :type "Actor Object Reference") (OtherComp :type "PrimitiveComponent Object Reference") (OtherBodyIndex :type Integer) (bFromSweep :type Boolean) (SweepResult :type "HitResult Structure (by ref)"))
  (bind _asplayer_painter (cast `/Game/blueprints/GameCharacter/PlayerPainter` (`GameplayStatics.GetPlayerPawn` 0)))
  (bind _equippedgun (`/Game/blueprints/GameCharacter/PlayerPainter.EquippedGun` _asplayer_painter))
  (set `/Game/blueprints/GunsBlueprint/BP_BaseGun.ammo` (+ (`/Game/blueprints/GunsBlueprint/BP_BaseGun.ammo` _equippedgun) 10) _equippedgun)
  (`self.K2_DestroyActor`)
  (`GameplayStatics.PlaySound2D` "/Game/Assets/slimejump-6913.slimejump-6913" 1.0 1.0 0.0 null null))

(fn `UserConstructionScript`)