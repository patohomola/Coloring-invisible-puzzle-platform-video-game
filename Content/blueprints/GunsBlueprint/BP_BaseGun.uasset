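; Base gun Blueprint that fires hitscan shots leaving randomly colored splats where they hit.
; Shoot checks CanShoot, deprojects the screen center into a ray, ignoring its location inputs, and passes it to BulletRaycast with a random hue.
; BulletRaycast runs a complex object trace and hands the result to ShooterPawn's TextureSplatDamage.
; It then clears CanShoot, which nothing in this graph resets.
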(fn `BulletRaycast`
  (params (Start :type "Vector Structure") (direction :type "Vector Structure") (distance :type "Float (double-precision)") (color :type "LinearColor Structure") (size :type "Float (double-precision)"))
  (bind (_outhit _returnvalue) (`KismetSystemLibrary.LineTraceSingleForObjects` Start (+ Start (* direction distance)) (`|MakeArray` "ObjectTypeQuery1" "ObjectTypeQuery2" "ObjectTypeQuery4" :!type "EObjectTypeQuery Enum") true))
  (bind _asshooter_pawn (cast `/Game/blueprints/ShooterPawn` (`GameplayStatics.GetPlayerPawn` 0)))
  (`/Game/blueprints/ShooterPawn.TextureSplatDamage` _asshooter_pawn _outhit _returnvalue color size)
  (set `self.canShoot` false))

(fn `Shoot`
  (params (StartLocation :type "Vector Structure") (EndLocation :type "Vector Structure"))
  (bind (_worldposition _worlddirection) (`GameplayStatics.DeprojectScreenToWorld` (`GameplayStatics.GetPlayerController` 0) (* (`WidgetLayoutLibrary.GetViewportSize`) 0.5)))
  (if (`self.canShoot`)
    (`self.BulletRaycast` _worldposition _worlddirection (`self.MaxBulletDistance`) (`KismetMathLibrary.HSVToRGB` (`KismetMathLibrary.RandomFloatInRange` 0.0 360.0) 1.0 1.0) (`self.ScaleOfSplat`))))

(fn `UserConstructionScript`)