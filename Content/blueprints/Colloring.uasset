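; Paint splat actor whose TextureSplatDamage draws colored splats onto hit surfaces and spawns a tinted Niagara effect.
; Each hit actor name maps to a render target, created on first hit at a power-of-two size from component bounds and bound to slot 0's dynamic material as damageRT.
; A dynamic brush material draws into it at the collision UV, using offset UV samples along random tangents to correct scale and squish.
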(event `self.ReceiveBeginPlay`
  (bind _returnvalue (`PrimitiveComponent.CreateDynamicMaterialInstance` (`self.Plane_Brush`) 0 "/Game/Painting/Splat_Paint_Brush.Splat_Paint_Brush" "None"))
  (set `self.brush` _returnvalue))

(fn `TextureSplatDamage`
  (params (hitlocartion :type "HitResult Structure") (ifHit :type Boolean) (color :type "LinearColor Structure") (size :type "Float (double-precision)"))
  (locals (HitObjectName :type String))
  (bind _brush (`self.brush`))
  (bind _uv (`GameplayStatics.FindCollisionUV` (`local.hitlocartion`)))
  (bind (_bblockinghit _binitialoverlap _time _distance _location _impactpoint _normal _impactnormal _physmat _hitactor _hitcomponent _hitbonename _bonename _hititem _elementindex _faceindex) (`GameplayStatics.BreakHitResult` (`local.hitlocartion`)))
  (bind (_bblockinghit_2 _binitialoverlap_2 _time_2 _distance_2 _location_2 _impactpoint_2 _normal_2) (`GameplayStatics.BreakHitResult` (`local.hitlocartion`)))
  (bind (_bblockinghit_3 _binitialoverlap_3 _time_3 _distance_3 _location_3 _impactpoint_3 _normal_3 _impactnormal_2 _physmat_2 _hitactor_2 _hitcomponent_2) (`GameplayStatics.BreakHitResult` (`local.hitlocartion`)))
  (bind (_bblockinghit_4 _binitialoverlap_4 _time_4 _distance_4 _location_4 _impactpoint_4 _normal_4 _impactnormal_3 _physmat_3 _hitactor_3) (`GameplayStatics.BreakHitResult` (`local.hitlocartion`)))
  (bind _returnvalue (`KismetMathLibrary.Normal` (`KismetMathLibrary.Cross_VectorVector` _normal_4 (`KismetMathLibrary.RandomUnitVectorFromStream` (`KismetMathLibrary.MakeRandomStream` (`KismetMathLibrary.FTrunc` _distance_4)))) 0.0))
  (bind _returnvalue_2 (`KismetMathLibrary.FTrunc` (`KismetMathLibrary.MultiplyMultiply_FloatFloat` 2.0 (`KismetMathLibrary.Conv_IntToDouble` (`KismetMathLibrary.FTrunc` (`KismetMathLibrary.MapRangeClamped` (/ (* (`KismetMathLibrary.Square` (`.SphereRadius` (`KismetSystemLibrary.GetComponentBounds` (`.HitComponent` (`GameplayStatics.BreakHitResult` (`local.hitlocartion`)))))) 12.0) 10000.0) 50.0 500.0 9.0 12.0))))))
  (bind _returnvalue_3 (- (`GameplayStatics.FindCollisionUV` (`GameplayStatics.MakeHitResult` false false 0.0 0.0 (+ _location (* _returnvalue 10.0)) (0.0 0.0 0.0) (0.0 0.0 1.0) (0.0 0.0 1.0) null null _hitcomponent "None" "None" 0 0 _faceindex)) _uv))
  (bind _returnvalue_4 (- (`GameplayStatics.FindCollisionUV` (`GameplayStatics.MakeHitResult` false false 0.0 0.0 (+ _location (* (`KismetMathLibrary.Normal` (`KismetMathLibrary.Cross_VectorVector` _returnvalue _normal_4) 0.0) 10.0)) (0.0 0.0 0.0) (0.0 0.0 1.0) (0.0 0.0 1.0) null null _hitcomponent "None" "None" 0 0 _faceindex)) _uv))
  (bind _returnvalue_5 (`KismetMathLibrary.MakeVector` (`KismetMathLibrary.DotProduct2D` _returnvalue_3 (1.0 0.0)) (`KismetMathLibrary.DotProduct2D` _returnvalue_4 (0.0 1.0))))
  (`|ExecutionSequence`
    (:`then_0`
      (set `local.HitObjectName` (`KismetSystemLibrary.GetObjectName` _hitactor_3)))
    (:`then_1`
      (if (`local.ifHit`)
        ;[1 1 1] is hit object in map?
        (if (`BlueprintMapLibrary.Map_Contains` (`self.MapNameToRT`) (`local.HitObjectName`))
          ;[1 1 1] draw damage
          (`MaterialInstanceDynamic.SetVectorParameterValue` _brush "uvTransform" (`KismetMathLibrary.Conv_VectorToLinearColor` (`KismetMathLibrary.Conv_Vector2DToVector` (`GameplayStatics.FindCollisionUV` (`local.hitlocartion`)))) :!label _label)
          (`MaterialInstanceDynamic.SetScalarParameterValue` _brush "scale" (`KismetMathLibrary.Sqrt` (* (/ -1.0 (+ (`KismetMathLibrary.Abs` (+ (.x (`KismetMathLibrary.Normal` _returnvalue_5 0.0)) (.y (`KismetMathLibrary.Normal` _returnvalue_5 0.0)))) -1.0)) (`KismetMathLibrary.CrossProduct2D` _returnvalue_4 _returnvalue_3) (`local.size`))))
          (`MaterialInstanceDynamic.SetVectorParameterValue` _brush "squish" (`KismetMathLibrary.Conv_VectorToLinearColor` _returnvalue_5))
          (`MaterialInstanceDynamic.SetScalarParameterValue` _brush "Frame" (`KismetMathLibrary.Conv_IntToDouble` (`KismetMathLibrary.RandomIntegerInRange` 0 3)))
          (`MaterialInstanceDynamic.SetVectorParameterValue` _brush "color" (`local.color`))
          (bind (_canvas _size) (`KismetRenderingLibrary.BeginDrawCanvasToRenderTarget` (`BlueprintMapLibrary.Map_Find` (`self.MapNameToRT`) (`local.HitObjectName`))))
          (`Canvas.K2_DrawMaterial` _canvas _brush (0.0 0.0) (`KismetMathLibrary.MakeVector2D` (`KismetMathLibrary.BreakVector2D` _size) (`.Y` (`KismetMathLibrary.BreakVector2D` _size))) (0.0 0.0) (1.0 1.0) 0.0 (0.5 0.5))
          (else
            (`|ExecutionSequence`
              (:`then_0`
                ;[1 1 1] new render material
                (bind _returnvalue_6 (`KismetRenderingLibrary.CreateRenderTarget2D` _returnvalue_2 _returnvalue_2))
                (`/Engine/EditorBlueprintResources/StandardMacros.IsValid` _returnvalue_6
                  (:`Is Valid`
                    (`BlueprintMapLibrary.Map_Add` (`self.MapNameToRT`) (`local.HitObjectName`) _returnvalue_6)
                    (bind _returnvalue_7 (`KismetMaterialLibrary.CreateDynamicMaterialInstance` (`PrimitiveComponent.GetMaterial` _hitcomponent_2 0)))
                    (`/Engine/EditorBlueprintResources/StandardMacros.IsValid` _returnvalue_7
                      (:`Is Valid`
                        (`PrimitiveComponent.SetMaterial` _hitcomponent_2 0 _returnvalue_7)
                        (`MaterialInstanceDynamic.SetTextureParameterValue` _returnvalue_7 "damageRT" _returnvalue_6))
                      (:`Is Not Valid`
                        (`KismetSystemLibrary.PrintText` "what2"))))
                  (:`Is Not Valid`
                    (`KismetSystemLibrary.PrintString` "fuck"))))
              (:`then_1`
                (goto _label)))))))
    (:`then_2`
      (bind _returnvalue_8 (`NiagaraFunctionLibrary.SpawnSystemAtLocation` "/Game/Painting/Particle/SplatSystem.SplatSystem" _location_2 (`KismetMathLibrary.Conv_VectorToRotator` _normal_2) (0.01 0.01 0.01)))
      (`NiagaraComponent.SetVariableLinearColor` _returnvalue_8 "color2" (`local.color`)))))

(fn `UserConstructionScript`)