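; Multi-shot gun Blueprint that fires a horizontal spread of bullet raycasts across the whole screen in one shot.
; When CanShoot is true, Shoot deprojects evenly spaced points along the screen's vertical midline height, ignoring its StartLocation and EndLocation inputs.
; Each point feeds BulletRaycast with MaxBulletDistance and a random fully saturated color.
; Tick calls the parent and prints the frame delta time.
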(event `self.ReceiveTick`
  (params (DeltaSeconds :type "Float (single-precision)"))
  (`parent.ReceiveTick` DeltaSeconds)
  (`KismetSystemLibrary.PrintText` (`KismetTextLibrary.Conv_DoubleToText` DeltaSeconds "HalfToEven")))

(fn `Shoot`
  (params (StartLocation :type "Vector Structure") (EndLocation :type "Vector Structure"))
  (bind (_returnvalue_x _returnvalue_y) (`KismetMathLibrary.BreakVector2D` (`WidgetLayoutLibrary.GetViewportSize`)))
  (if (`self.canShoot`)
    (for _index (range 11)
      (bind (_worldposition _worlddirection) (`GameplayStatics.DeprojectScreenToWorld` (`GameplayStatics.GetPlayerController` 0) (* (`KismetMathLibrary.MakeVector2D` _returnvalue_x _returnvalue_y) (`KismetMathLibrary.MakeVector2D` (/ _index 10) 0.5))))
      (`self.BulletRaycast` _worldposition _worlddirection (`self.MaxBulletDistance`) (`KismetMathLibrary.HSVToRGB` (`KismetMathLibrary.RandomFloatInRange` 0.0 360.0) 1.0 1.0) 5.0))))

(fn `UserConstructionScript`
  (`parent.UserConstructionScript`))