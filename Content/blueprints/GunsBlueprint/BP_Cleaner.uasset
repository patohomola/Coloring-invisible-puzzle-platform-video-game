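; BP_Cleaner is a gun Blueprint that fires white splats, which its name suggests serve as a cleaning shot.
; Shoot deprojects the viewport center into a world ray, passes it to BulletRaycast with the gun's range and splat size, then clears CanShoot.
; Shoot_0 is empty apart from a disconnected random-hue variant of the same shot, and the event graph holds only disabled stubs.
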(fn `Shoot`
  (params (StartLocation :type "Vector Structure") (EndLocation :type "Vector Structure"))
  (bind (_worldposition _worlddirection) (`GameplayStatics.DeprojectScreenToWorld` (`GameplayStatics.GetPlayerController` 0) (* (`WidgetLayoutLibrary.GetViewportSize`) 0.5)))
  (`self.BulletRaycast` _worldposition _worlddirection (`self.MaxBulletDistance`) (`KismetMathLibrary.MakeColor` 1.0 1.0 1.0) (`self.ScaleOfSplat`))
  (set `self.canShoot` false))

(fn `Shoot_0`
  (params (StartLocation :type "Vector Structure" :default (0.0 0.0 0.0)) (EndLocation :type "Vector Structure" :default (0.0 0.0 0.0))))

(fn `UserConstructionScript`
  (`parent.UserConstructionScript`))