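; Player controller that shows the Countdown widget on begin play and handles movement, look and jump input for the controlled pawn.
; It adds the IM_Main Enhanced Input context; IA_movement moves the pawn relative to its forward and right vectors.
; Legacy axis bindings drive yaw and pitch.
; A hard-coded SpaceBar key jumps by setting the ShooterPawn's VerticalImersia and clearing IsOnGround, only when grounded.
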(event `self.ReceiveBeginPlay`
  (bind _returnvalue (pcsubsystem `EnhancedInputLocalPlayerSubsystem` self))
  ;[1 1 1] Initialization
  (`|ExecutionSequence`
    (:`then_0`
      (bind _returnvalue_2 (`|CreateWidget` "/Game/gameUI/Countdown.Countdown_C"))
      (`UserWidget.AddToViewport` _returnvalue_2 0)
      (set `self.coundown` _returnvalue_2))
    (:`then_1`
      (`/Engine/EditorBlueprintResources/StandardMacros.IsValid` _returnvalue
        (:`Is Valid`
          (`EnhancedInputSubsystemInterface.AddMappingContext` _returnvalue "/Game/input/IM_Main.IM_Main" 0 (struct)))))))

(event `EnhancedInput|/Game/input/inputAction/IA_movement`
  (params (ActionValue :type "Vector2D Structure") (ElapsedSeconds :type "Float (double-precision)") (TriggeredSeconds :type "Float (double-precision)") (InputAction :type "InputAction Object Reference" :default "/Game/input/inputAction/IA_movement.IA_movement"))
  (:`Triggered`
    (`Pawn.AddMovementInput` (`self.K2_GetPawn`) (`self.Movement direction` ActionValue) 1.0 false)))

(event `InputAxis|LoopAround`
  (params (AxisValue :type "Float (single-precision)"))
  (`self.AddYawInput` AxisValue))

(event `InputAxis|LoopUP`
  (params (AxisValue :type "Float (single-precision)"))
  (`self.AddPitchInput` AxisValue))

(event `Key|SpaceBar`
  (params (Key :type "Key Structure"))
  (:`Pressed`
    (bind _asshooter_pawn (cast `/Game/blueprints/GameCharacter/ShooterPawn` (`GameplayStatics.GetPlayerPawn` 0)))
    (if (`/Game/blueprints/GameCharacter/ShooterPawn.isOnGround` _asshooter_pawn)
      (set `/Game/blueprints/GameCharacter/ShooterPawn.verticalImersia` 250.0 _asshooter_pawn)
      (set `/Game/blueprints/GameCharacter/ShooterPawn.isOnGround` false _asshooter_pawn))))

(fn `Movement direction`
  (params (InVec :type "Vector2D Structure"))
  (returns (ReturnValue :type "Vector Structure"))
  (bind _returnvalue (`self.K2_GetPawn`))
  (bind (_x _y) (`KismetMathLibrary.BreakVector2D` InVec))
  (return (+ (* (`self.GetActorRightVector` _returnvalue) _x) (* (`self.GetActorForwardVector` _returnvalue) _y))))

(fn `UserConstructionScript`)