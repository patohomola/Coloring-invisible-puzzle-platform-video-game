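; Manager Blueprint that awards countdown time and triggers game over through the player's BP_controller.
; AddTime increments the controller countdown's room count, then adds the input time divided by a base-5 logarithm of that count plus an offset, so bonuses shrink as rooms accumulate.
; GameOver forwards to the controller's GameOver, and both events play a 2D sound cue.
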(event `self.AddTime`
  (params (InputValue :type Integer))
  (bind _returnvalue (+ 5.0 0.0))
  (`KismetSystemLibrary.PrintText` (`KismetTextLibrary.Conv_IntToText` InputValue))
  (bind _asbp_controller (cast `/Game/blueprints/GameCharacter/BP_controller` (`GameplayStatics.GetPlayerController` 0)))
  (bind _coundown (`/Game/blueprints/GameCharacter/BP_controller.coundown` _asbp_controller))
  (bind _roomcount (`/Game/gameUI/Countdown.roomCount` _coundown))
  (`/Engine/EditorBlueprintResources/StandardMacros.IncrementInt` _roomcount
    (:`  `
      (set `/Game/gameUI/Countdown.countDown` (+ (`/Game/gameUI/Countdown.countDown` _coundown) (/ (`KismetMathLibrary.Conv_IntToDouble` InputValue) (`KismetMathLibrary.Log` (+ (`KismetMathLibrary.Conv_IntToDouble` _roomcount) -1.0 _returnvalue) _returnvalue))) _coundown)
      (`GameplayStatics.PlaySound2D` "/Game/Assets/success2-57646.success2-57646" 1.0 1.0 0.0 null null))))

(event `self.GameOver`
  (params (InputValue :type Integer))
  (bind _asbp_controller (cast `/Game/blueprints/GameCharacter/BP_controller` (`GameplayStatics.GetPlayerController` 0)))
  (`/Game/blueprints/GameCharacter/BP_controller.GameOver` _asbp_controller)
  (`GameplayStatics.PlaySound2D` "/Game/Assets/splash-by-blaukreuz-6261.splash-by-blaukreuz-6261" 1.0 1.0 0.0 null null))

(fn `UserConstructionScript`)