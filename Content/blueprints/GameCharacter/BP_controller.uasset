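; Player controller that manages the countdown HUD, pause menu and game-over screen.
; On BeginPlay it shows a Countdown widget and adds the IM_Main Enhanced Input mapping context.
; The PauseMenu input and GameOver function pause the game, open their widget with UI-only input and cursor, and remove the countdown; GameOver also passes it to LoadScore.
; UnPause only re-adds the countdown to the viewport.
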(event `self.ReceiveBeginPlay`
  (bind _returnvalue (pcsubsystem `EnhancedInputLocalPlayerSubsystem` self))
  ;[1 1 1] Initialization
  (`|ExecutionSequence`
    (:`then_0`
      (bind _returnvalue_2 (`|CreateWidget` "/Game/gameUI/Countdown.Countdown_C"))
      (`UserWidget.AddToViewport` _returnvalue_2 0)
      (set `self.coundown` _returnvalue_2))
    (:`then_1`
      (`/Engine/EditorBlueprintResources/StandardMacros.IsValid` _returnvalue
        (:`Is Valid`
          (`EnhancedInputSubsystemInterface.AddMappingContext` _returnvalue "/Game/input/IM_Main.IM_Main" 0 (struct)))))))

(event `EnhancedInput|/Game/input/inputAction/PauseMenu`
  (params (ActionValue :type Boolean) (ElapsedSeconds :type "Float (double-precision)") (TriggeredSeconds :type "Float (double-precision)") (InputAction :type "InputAction Object Reference" :default "/Game/input/inputAction/PauseMenu.PauseMenu"))
  (:`Triggered`
    (`GameplayStatics.SetGamePaused` true)
    (bind _returnvalue (`|CreateWidget` "/Game/gameUI/PauseMenu.PauseMenu_C"))
    (`UserWidget.AddToViewport` _returnvalue 0)
    (set `self.bShowMouseCursor` true)
    (`WidgetBlueprintLibrary.SetInputMode_UIOnlyEx` self _returnvalue)
    (`Widget.RemoveFromParent` (`self.coundown`))))

(event `UnPause`
  (`UserWidget.AddToViewport` (`self.coundown`) 0))

(fn `GameOver`
  (bind _returnvalue (`|CreateWidget` "/Game/gameUI/WB_gameOver.WB_gameOver_C"))
  (`UserWidget.AddToViewport` _returnvalue 0)
  (set `self.bShowMouseCursor` true)
  (`WidgetBlueprintLibrary.SetInputMode_UIOnlyEx` self _returnvalue)
  (`/Game/gameUI/WB_gameOver.LoadScore` _returnvalue (`self.coundown`))
  (`Widget.RemoveFromParent` (`self.coundown`))
  (`GameplayStatics.SetGamePaused` true))

(fn `UserConstructionScript`)