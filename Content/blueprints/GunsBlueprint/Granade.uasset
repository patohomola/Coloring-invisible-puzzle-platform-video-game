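; Paint grenade that bursts two seconds after BeginPlay, spraying randomly colored splats onto surrounding geometry.
; A delayed DoN loop fires 100 rapid RandomPaf shots, each printing "bum" and tracing from Sphere1 in a random, unnormalized direction with a random hue.
; BulletRaycast line-traces against static, dynamic and physics objects, passing results to TextureSplatDamage on the Colloring actor found at startup.
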(event `self.ReceiveBeginPlay`
  (bind _returnvalue (`GameplayStatics.GetActorOfClass` "/Game/Painting/Colloring.Colloring_C"))
  (set `self.wordCanvas` _returnvalue)
  (`KismetSystemLibrary.Delay` 2.0)
  (`/Engine/EditorBlueprintResources/StandardMacros.Do N` 100 :!label _label
    (:`Exit`
      (`self.random paf`)
      (`KismetSystemLibrary.Delay` 0.002)
      (goto _label))))

(fn `BulletRaycast`
  (params (Start :type "Vector Structure") (direction :type "Vector Structure") (distance :type "Float (double-precision)") (color :type "LinearColor Structure") (size :type "Float (double-precision)"))
  (bind (_outhit _returnvalue) (`KismetSystemLibrary.LineTraceSingleForObjects` Start (+ Start (* direction distance)) (`|MakeArray` "ObjectTypeQuery1" "ObjectTypeQuery2" "ObjectTypeQuery4" :!type "EObjectTypeQuery Enum") true))
  (`/Game/Painting/Colloring.TextureSplatDamage` (`self.wordCanvas`) _outhit _returnvalue (`local.color`) (`local.size`) false))

(fn `random paf`
  (`KismetSystemLibrary.PrintText` "bum")
  (`self.BulletRaycast` (`SceneComponent.K2_GetComponentLocation` (`self.Sphere1`)) (* (`KismetMathLibrary.MakeVector` (`KismetMathLibrary.RandomFloatInRange` -1.0 1.0) (`KismetMathLibrary.RandomFloatInRange` -1.0 1.0) (`KismetMathLibrary.RandomFloatInRange` -1.0 1.0)) (`KismetMathLibrary.GetPI`)) 1000.0 (`KismetMathLibrary.HSVToRGB` (`KismetMathLibrary.RandomFloatInRange` 0.0 360.0) 1.0 1.0) 5.0))

(fn `UserConstructionScript`)