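; Grenade launcher weapon Blueprint that fires a Granade actor along the player's view.
; Shoot, gated by CanShoot, spawns a scaled-down Granade at the Ammo0 component using player 0's camera rotation, ignoring its start and end inputs.
; It then clears CanShoot, which nothing in these graphs resets.
; The forward spawn offset is zero, the firing sound is disconnected, and the event graph and NewFunction are empty stubs.
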(fn `NewFunction`)

(fn `Shoot`
  (params (StartLocation :type "Vector Structure") (EndLocation :type "Vector Structure"))
  (bind _returnvalue (`PlayerCameraManager.GetCameraRotation` (`GameplayStatics.GetPlayerCameraManager` 0)))
  (if (`self.canShoot`)
    (`|SpawnActorFromClass` "/Game/blueprints/GunsBlueprint/Granade.Granade_C" (`KismetMathLibrary.MakeTransform` (+ (`SceneComponent.K2_GetComponentLocation` (`self.ammo_0`)) (`KismetMathLibrary.GreaterGreater_VectorRotator` (0.0 0.0 0.0) _returnvalue)) _returnvalue (`KismetMathLibrary.Conv_DoubleToVector` 0.2)) "Undefined" "OverrideRootScale" null null)
    (set `self.canShoot` false)))

(fn `UserConstructionScript`
  (`parent.UserConstructionScript`))