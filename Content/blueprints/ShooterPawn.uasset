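; Player shooter pawn that fires a spawned paint gun and can paint splats onto hit surfaces.
; Tick applies swept movement input, hand-rolled gravity and controller yaw and pitch, while Shoot resets the gun after its fire-rate delay.
; TextureSplatDamage lazily creates a bounds-sized render target per hit actor, feeding its material's damageRT.
; It draws a brush material at the hit UV, sampling nearby UVs to correct splat scale and squish.
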(event `self.ReceiveTick`
  (params (DeltaSeconds :type "Float (single-precision)"))
  (bind _verticalimersia (`self.verticalImersia`))
  (bind (_returnvalue_roll _returnvalue_pitch _returnvalue_yaw) (`KismetMathLibrary.BreakRotator` (`self.K2_GetActorRotation` (`GameplayStatics.GetPlayerController` 0))))
  (bind _returnvalue (`self.ConsumeMovementInputVector`))
  (`self.K2_AddActorWorldOffset` (* _returnvalue (`self.speed`) DeltaSeconds) true)
  (`self.K2_SetActorRotation` (`KismetMathLibrary.MakeRotator` 0.0 0.0 _returnvalue_yaw))
  (`SceneComponent.K2_SetRelativeLocationAndRotation` (`self.Camera`) (0.0 0.0 0.0) (`KismetMathLibrary.MakeRotator` 0.0 _returnvalue_pitch) false false)
  (bind _sweephitresult (`self.K2_AddActorWorldOffset` (`KismetMathLibrary.MakeVector` 0.0 0.0 (* _verticalimersia DeltaSeconds)) true))
  (set `self.verticalImersia` (+ _verticalimersia (* DeltaSeconds -250.0)))
  (if (`GameplayStatics.BreakHitResult` _sweephitresult)
    (set `self.isOnGround` (< (`self.verticalImersia`) 0.0))
    (set `self.verticalImersia` 0.0)))

(event `self.ReceiveBeginPlay`
  (bind _returnvalue (`PrimitiveComponent.CreateDynamicMaterialInstance` (`self.Sphere`) 0 "/Game/Painting/Splat_Paint_Brush.Splat_Paint_Brush" "None"))
  (set `self.brush` _returnvalue)
  (bind _returnvalue_2 (`|SpawnActorFromClass` "/Game/blueprints/GunsBlueprint/BP_DefaultPaintGun.BP_DefaultPaintGun_C" (`KismetMathLibrary.MakeTransform` (0.0 0.0 0.0)) "Undefined" "MultiplyWithRoot" null null))
  (bind _output_get (set `self.EquippedGun` _returnvalue_2))
  (`self.K2_AttachToComponent` _output_get (`self.Gun location`) "None" "KeepRelative" "KeepRelative" "KeepRelative" true))

(event `InputAction|shoot`
  (params (Key :type "Key Structure")))

(event `EnhancedInput|/Game/input/inputAction/Shoot`
  (params (ActionValue :type Boolean) (ElapsedSeconds :type "Float (double-precision)") (TriggeredSeconds :type "Float (double-precision)") (InputAction :type "InputAction Object Reference" :default "/Game/input/inputAction/Shoot.Shoot"))
  (bind _equippedgun (`self.EquippedGun`))
  (:`Triggered`
    (`/Game/blueprints/GunsBlueprint/BP_BaseGun.Shoot` _equippedgun (0.0 0.0 0.0) (0.0 0.0 0.0))
    (`KismetSystemLibrary.Delay` (`/Game/blueprints/GunsBlueprint/BP_BaseGun.FireRate` _equippedgun))
    (set `/Game/blueprints/GunsBlueprint/BP_BaseGun.canShoot` true _equippedgun)))

(fn `TextureSplatDamage`
  (params (hitlocartion :type "HitResult Structure") (ifHit :type Boolean) (color :type "LinearColor Structure") (size :type "Float (double-precision)"))
  (locals (`splat size` :type "Float (double-precision)") (splat_color :type "LinearColor Structure"))
  (bind _uv (`GameplayStatics.FindCollisionUV` hitlocartion))
  (bind (_bblockinghit _binitialoverlap _time _distance _location _impactpoint _normal _impactnormal _physmat _hitactor _hitcomponent _hitbonename _bonename _hititem _elementindex _faceindex) (`GameplayStatics.BreakHitResult` hitlocartion))
  (bind _brush (`self.brush`))
  (bind _returnvalue (`KismetSystemLibrary.GetObjectName` _hitactor))
  (bind _returnvalue_2 (`KismetMathLibrary.Normal` (`KismetMathLibrary.Cross_VectorVector` _normal (`KismetMathLibrary.RandomUnitVectorFromStream` (`KismetMathLibrary.MakeRandomStream` (`KismetMathLibrary.FTrunc` _distance)))) 0.0))
  (bind _returnvalue_3 (`KismetMathLibrary.FTrunc` (`KismetMathLibrary.MultiplyMultiply_FloatFloat` 2.0 (`KismetMathLibrary.Conv_IntToDouble` (`KismetMathLibrary.FTrunc` (`KismetMathLibrary.MapRangeClamped` (/ (* (`KismetMathLibrary.Square` (`.SphereRadius` (`KismetSystemLibrary.GetComponentBounds` _hitcomponent))) 12.0) 10000.0) 50.0 500.0 8.0 12.0))))))
  (bind _returnvalue_4 (- (`GameplayStatics.FindCollisionUV` (`GameplayStatics.MakeHitResult` false false 0.0 0.0 (+ _location (* _returnvalue_2 10.0)) (0.0 0.0 0.0) (0.0 0.0 1.0) (0.0 0.0 1.0) null null _hitcomponent "None" "None" 0 0 _faceindex)) _uv))
  (bind _returnvalue_5 (- (`GameplayStatics.FindCollisionUV` (`GameplayStatics.MakeHitResult` false false 0.0 0.0 (+ _location (* (`KismetMathLibrary.Normal` (`KismetMathLibrary.Cross_VectorVector` _returnvalue_2 _normal) 0.0) 10.0)) (0.0 0.0 0.0) (0.0 0.0 1.0) (0.0 0.0 1.0) null null _hitcomponent "None" "None" 0 0 _faceindex)) _uv))
  (bind _returnvalue_6 (`KismetMathLibrary.MakeVector` (`KismetMathLibrary.DotProduct2D` _returnvalue_4 (1.0 0.0)) (`KismetMathLibrary.DotProduct2D` _returnvalue_5 (0.0 1.0))))
  (set `local.splat size` size)
  (set `local.splat_color` color)
  (`|ExecutionSequence`
    (:`then_0`
      (if ifHit
        ;[1 1 1] is hit object in map?
        (if (`BlueprintMapLibrary.Map_Contains` (`self.MapNameToRT`) _returnvalue)
          ;[1 1 1] draw damage
          (`MaterialInstanceDynamic.SetVectorParameterValue` _brush "uvTransform" (`KismetMathLibrary.Conv_VectorToLinearColor` (`KismetMathLibrary.Conv_Vector2DToVector` _uv)) :!label _label)
          (`MaterialInstanceDynamic.SetScalarParameterValue` _brush "scale" (`KismetMathLibrary.Sqrt` (* (/ -1.0 (+ (`KismetMathLibrary.Abs` (+ (.x (`KismetMathLibrary.Normal` _returnvalue_6 0.0)) (.y (`KismetMathLibrary.Normal` _returnvalue_6 0.0)))) -1.0)) (`KismetMathLibrary.CrossProduct2D` _returnvalue_5 _returnvalue_4) (`local.splat size`))))
          (`MaterialInstanceDynamic.SetVectorParameterValue` _brush "squish" (`KismetMathLibrary.Conv_VectorToLinearColor` _returnvalue_6))
          (`MaterialInstanceDynamic.SetScalarParameterValue` _brush "Frame" (`KismetMathLibrary.Conv_IntToDouble` (`KismetMathLibrary.RandomIntegerInRange` 0 3)))
          (`MaterialInstanceDynamic.SetVectorParameterValue` _brush "color" (`local.splat_color`))
          (bind (_canvas _size) (`KismetRenderingLibrary.BeginDrawCanvasToRenderTarget` (`BlueprintMapLibrary.Map_Find` (`self.MapNameToRT`) _returnvalue)))
          (`Canvas.K2_DrawMaterial` _canvas _brush (0.0 0.0) (`KismetMathLibrary.MakeVector2D` (`KismetMathLibrary.BreakVector2D` _size) (`.Y` (`KismetMathLibrary.BreakVector2D` _size))) (0.0 0.0) (1.0 1.0) 0.0 (0.5 0.5))
          (else
            (`|ExecutionSequence`
              (:`then_0`
                ;[1 1 1] new render material
                (bind _returnvalue_7 (`KismetRenderingLibrary.CreateRenderTarget2D` _returnvalue_3 _returnvalue_3))
                (`/Engine/EditorBlueprintResources/StandardMacros.IsValid` _returnvalue_7
                  (:`Is Valid`
                    (if true
                      (`BlueprintMapLibrary.Map_Add` (`self.MapNameToRT`) _returnvalue _returnvalue_7)
                      (bind _returnvalue_8 (`KismetMaterialLibrary.CreateDynamicMaterialInstance` (`PrimitiveComponent.GetMaterial` _hitcomponent 0)))
                      (`/Engine/EditorBlueprintResources/StandardMacros.IsValid` _returnvalue_8
                        (:`Is Valid`
                          (`PrimitiveComponent.SetMaterial` _hitcomponent 0 _returnvalue_8)
                          (`MaterialInstanceDynamic.SetTextureParameterValue` _returnvalue_8 "damageRT" _returnvalue_7))
                        (:`Is Not Valid`
                          (`KismetSystemLibrary.PrintText` "what2")))))
                  (:`Is Not Valid`
                    (`KismetSystemLibrary.PrintString` "fuck"))))
              (:`then_1`
                (goto _label)))))))))

(fn `UserConstructionScript`)